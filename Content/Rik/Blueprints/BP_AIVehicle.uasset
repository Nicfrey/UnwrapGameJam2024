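; Player-input vehicle pawn, despite the AIVehicle name, that drives itself forward while IA_Movement steers its yaw and front-left wheel.
; Each Tick moves it with a swept offset, drains health and fuel, and prints health; wheel health stays unchanged.
; Speed scales down below half health, and zero health triggers one-time fire, explosion and sound effects.
; Running out of fuel opens the DrivingTests level.
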(event EventBeginPlay
  (CallFunction|InitVehicleAttributes)
  (bind _asplayer_controller (Utilities|Casting|CastToPlayerController (Pawn|GetController)))
  (Utilities|IsValid (PlayerController|LocalPlayerSubsystems|GetEnhancedInputLocalPlayerSubsystem _asplayer_controller)
    (:Is%20Valid
      (Input|AddMappingContext (PlayerController|LocalPlayerSubsystems|GetEnhancedInputLocalPlayerSubsystem _asplayer_controller) "/Game/Alexandre/Blueprints/MC_Movement.MC_Movement" 0 "(bIgnoreAllPressedKeysUntilRelease=True,bForceImmediately=False)"))))

(event Collision|EventActorBeginOverlap
  (params (OtherActor :type Actor%20Object%20Reference)))

(event EventTick
  (params (DeltaSeconds :type Float%20%28single-precision%29))
  (CallFunction|RotateWheels)
  ;[1 1 1] Rotation
  (Class|Actor|AddActorWorldRotation (Math|Rotator|MakeRotator 0.0 0.0 (* (* DeltaSeconds (Variables|VehicleMovement|GetRotationSpeed)) (Input|EnhancedActionValues|GetIA_Movement))))
  ;[1 1 1] Discplacement
  (Transformation|AddActorWorldOffset (* (Math|Vector|GetForwardVector (Variables|Default|GetBody)) (* (Variables|VehicleMovement|GetCurrentSpeed) (Utilities|Time|GetWorldDeltaSeconds))) true)
  (CallFunction|DecrementVehicleAttributes)
  (CallFunction|CheckforLowAmount)
  (Development|PrintString (Utilities|String|ToString(Float) (Variables|VehicleAttributes|GetCurrentHealth)))
  (if (<= (Variables|VehicleAttributes|GetCurrentHealth) 0.0)
    (Utilities|FlowControl|DoOnce false
      (:Completed
        (Effects|SpawnEmitteratLocation "/Game/StarterContent/Particles/P_Fire.P_Fire" (Transformation|GetActorLocation) "0, 0, 0" "1.000000,1.000000,1.000000" false)
        (Effects|SpawnEmitteratLocation "/Game/StarterContent/Particles/P_Explosion.P_Explosion" (Transformation|GetActorLocation))
        (Audio|PlaySound2D "/Game/StarterContent/Audio/Explosion_Cue.Explosion_Cue" 1.0 1.0 0.0 0 0)))))

(fn ConstructionScript)

(fn InitVehicleAttributes
  (Variables|VehicleAttributes|SetCurrentHealth (Variables|VehicleAttributes|GetMaxHealth))
  (Variables|VehicleAttributes|SetCurrentFuel (Variables|VehicleAttributes|GetMaxFuel)))

(fn DecrementVehicleAttributes
  (CallFunction|ChangeHealth (* (* (Variables|VehicleAttributes|GetHealthLoosingSpeed) (Utilities|Time|GetWorldDeltaSeconds)) -1.0))
  (CallFunction|ChangeFuelValue (* (* (Variables|VehicleAttributes|GetFuelLoosingSpeed) (Utilities|Time|GetWorldDeltaSeconds)) -1.0))
  (CallFunction|ChangeWheelsHealth 0.0))

(fn ChangeHealth
  (params (ChangingValue :type Float%20%28double-precision%29))
  (Variables|VehicleAttributes|SetCurrentHealth (+ ChangingValue (Variables|VehicleAttributes|GetCurrentHealth)))
  (Utilities|FlowControl|Sequence
    (:then_0
      (if (< (Variables|VehicleAttributes|GetCurrentHealth) 0.0)
        (Variables|VehicleAttributes|SetCurrentHealth 0.0)))
    (:then_1
      (if (> (Variables|VehicleAttributes|GetCurrentHealth) (Variables|VehicleAttributes|GetMaxHealth))
        (Variables|VehicleAttributes|SetCurrentHealth (Variables|VehicleAttributes|GetMaxHealth))))))

(fn ChangeFuelValue
  (params (ChangingValue :type Float%20%28double-precision%29))
  (Variables|VehicleAttributes|SetCurrentFuel (+ ChangingValue (Variables|VehicleAttributes|GetCurrentFuel)))
  (Utilities|FlowControl|Sequence
    (:then_0
      (if (< (Variables|VehicleAttributes|GetCurrentFuel) 0.0)
        (Variables|VehicleAttributes|SetCurrentFuel 0.0)))
    (:then_1
      (if (> (Variables|VehicleAttributes|GetCurrentFuel) (Variables|VehicleAttributes|GetMaxFuel))
        (Variables|VehicleAttributes|SetCurrentFuel (Variables|VehicleAttributes|GetMaxFuel))))))

(fn ChangeWheelsHealth
  (params (ChangingValue :type Float%20%28double-precision%29))
  (Variables|VehicleAttributes|SetCurrentWheelHealth (+ ChangingValue (Variables|VehicleAttributes|GetCurrentWheelHealth)))
  (Utilities|FlowControl|Sequence
    (:then_0
      (if (< (Variables|VehicleAttributes|GetCurrentWheelHealth) 0.0)
        (Variables|VehicleAttributes|SetCurrentWheelHealth 0.0)))
    (:then_1
      (if (> (Variables|VehicleAttributes|GetCurrentWheelHealth) (Variables|VehicleAttributes|GetMaxWheelHealth))
        (Variables|VehicleAttributes|SetCurrentWheelHealth (Variables|VehicleAttributes|GetMaxWheelHealth))))))

(fn RotateWheels
  (bind _flwheel (Variables|Default|GetFLWheel))
  (bind _flwheel_2 (Variables|Default|GetFLWheel))
  (bind _flwheel_3 (Variables|Default|GetFLWheel))
  (bind _flwheel_4 (Variables|Default|GetFLWheel))
  (bind _relativerotation (Variables|/Script/Engine.SceneComponent|GetRelativeRotation _flwheel_3))
  (bind _relativerotation_2 (Variables|/Script/Engine.SceneComponent|GetRelativeRotation _flwheel_2))
  (bind _relativerotation_3 (Variables|/Script/Engine.SceneComponent|GetRelativeRotation _flwheel))
  (bind _relativerotation_4 (Variables|/Script/Engine.SceneComponent|GetRelativeRotation _flwheel_4))
  (if (and (> (Input|EnhancedActionValues|GetIA_Movement) 0.0) (< (.yaw (Variables|/Script/Engine.SceneComponent|GetRelativeRotation (Variables|Default|GetFLWheel))) (+ (Variables|Wheels|GetWheelMaxRotation) (Variables|Wheels|GetWheelStartRotation))))
    (Transformation|SetRelativeRotation (Variables|Default|GetFLWheel) (Math|Rotator|MakeRotator (.roll _relativerotation_3) (.pitch _relativerotation_3) (+ (.yaw _relativerotation_3) (Variables|Wheels|GetWheelRotatingSpeed))) false false)
    (elif (and (< (Input|EnhancedActionValues|GetIA_Movement) 0.0) (> (.yaw (Variables|/Script/Engine.SceneComponent|GetRelativeRotation (Variables|Default|GetFLWheel))) (- (Variables|Wheels|GetWheelStartRotation) (Variables|Wheels|GetWheelMaxRotation))))
      (Transformation|SetRelativeRotation (Variables|Default|GetFLWheel) (Math|Rotator|MakeRotator (.roll _relativerotation_2) (.pitch _relativerotation_2) (+ (.yaw _relativerotation_2) (* (Variables|Wheels|GetWheelRotatingSpeed) -1.0))) false false)
      (elif (> (.yaw (Variables|/Script/Engine.SceneComponent|GetRelativeRotation (Variables|Default|GetFLWheel))) (Variables|Wheels|GetWheelStartRotation))
        (Transformation|SetRelativeRotation (Variables|Default|GetFLWheel) (Math|Rotator|MakeRotator (.roll _relativerotation_4) (.pitch _relativerotation_4) (+ (.yaw _relativerotation_4) (* (Variables|Wheels|GetWheelRotatingSpeed) -1.0))) false false)
        (elif (< (.yaw (Variables|/Script/Engine.SceneComponent|GetRelativeRotation (Variables|Default|GetFLWheel))) (Variables|Wheels|GetWheelStartRotation))
          (Transformation|SetRelativeRotation (Variables|Default|GetFLWheel) (Math|Rotator|MakeRotator (.roll _relativerotation) (.pitch _relativerotation) (+ (.yaw _relativerotation) (Variables|Wheels|GetWheelRotatingSpeed))) false false))))))

(fn CheckforLowAmount
  (Utilities|FlowControl|Sequence
    (:then_0
      ;[1 1 1] Out Of Fuel
      (if (<= (Variables|VehicleAttributes|GetCurrentFuel) 0.0)
        (Game|OpenLevel(byName) "DrivingTests")))
    (:then_1
      (Variables|VehicleMovement|SetCurrentSpeed (Math|Float|SelectFloat (Variables|VehicleMovement|GetMaxSpeed) (* (/ (Variables|VehicleAttributes|GetCurrentHealth) (/ (Variables|VehicleAttributes|GetMaxHealth) 2.0)) (Variables|VehicleMovement|GetMaxSpeed)) (> (Variables|VehicleAttributes|GetCurrentHealth) (/ (Variables|VehicleAttributes|GetMaxHealth) 2.0)))))))