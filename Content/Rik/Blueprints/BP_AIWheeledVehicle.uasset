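; An AI wheeled vehicle that constantly drives toward the player's pawn.
; It sets full throttle once on BeginPlay and never adjusts it.
; Each tick it maps the yaw difference between its heading and the player's direction to a clamped steering input, scaled by Steering.
; It also passes forward speed to BPResetPos every tick to reset its position if stuck.
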(event EventBeginPlay
  (Class|ChaosVehicleMovementComponent|SetThrottleInput (Variables|Default|GetVehicleMovementComponent) 1.0))

(event EventTick
  (params (DeltaSeconds :type Float%20%28single-precision%29))
  (Class|ChaosVehicleMovementComponent|SetSteeringInput (Variables|Default|GetVehicleMovementComponent) (* (Math|Float|MapRangeClamped (.yaw (Math|Rotator|Delta(Rotator) (Math|Rotator|FindLookatRotation (Transformation|GetActorLocation) (Transformation|GetActorLocation (Game|Player|GetPlayerPawn 0))) (Transformation|GetActorRotation))) -9e+01 9e+01 -1.0 1.0) (Variables|Default|GetSteering)))
  (Default|ResetPosifStuck (Variables|Default|GetBP_ResetPos) (Vehicle|GetForwardSpeed (Variables|Default|GetVehicleMovementComponent))))

(fn ConstructionScript)