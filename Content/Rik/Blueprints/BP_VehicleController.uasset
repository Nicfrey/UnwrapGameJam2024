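; Player controller for a drivable vehicle that turns Enhanced Input throttle and steering into vehicle state.
; On BeginPlay it adds the default input mapping context and caches the controlled pawn as a BP_BaseVehicle.
; While input triggers, it smoothly interpolates the vehicle's current speed and steering angle toward the input value scaled by that vehicle's maximums.
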(event Input|EnhancedActionEvents|EnhancedInputActionIA_Steer
  (params (ActionValue :type Float%20%28double-precision%29) (ElapsedSeconds :type Float%20%28double-precision%29) (TriggeredSeconds :type Float%20%28double-precision%29) (InputAction :type Input%20Action%20Object%20Reference :default "/Game/Rik/Input/Actions/IA_Steer.IA_Steer"))
  (:Triggered
    (Variables|/Game/Rik/Blueprints/BP_BaseVehicle.BP_BaseVehicle_C|SetCurrentSteeringAngle (Variables|Default|GetVehicle) (Math|Interpolation|FInterpTo (Variables|/Game/Rik/Blueprints/BP_BaseVehicle.BP_BaseVehicle_C|GetCurrentSteeringAngle (Variables|Default|GetVehicle)) (* ActionValue (Variables|/Game/Rik/Blueprints/BP_BaseVehicle.BP_BaseVehicle_C|GetMaximumSteeringAngle (Variables|Default|GetVehicle))) (Utilities|Time|GetWorldDeltaSeconds) 4.0))))

(event Input|EnhancedActionEvents|EnhancedInputActionIA_Throttle
  (params (ActionValue :type Float%20%28double-precision%29) (ElapsedSeconds :type Float%20%28double-precision%29) (TriggeredSeconds :type Float%20%28double-precision%29) (InputAction :type Input%20Action%20Object%20Reference :default "/Game/Rik/Input/Actions/IA_Throttle.IA_Throttle"))
  (:Triggered
    (Variables|/Game/Rik/Blueprints/BP_BaseVehicle.BP_BaseVehicle_C|SetCurrentSpeed (Variables|Default|GetVehicle) (Math|Interpolation|FInterpTo (Variables|/Game/Rik/Blueprints/BP_BaseVehicle.BP_BaseVehicle_C|GetCurrentSpeed (Variables|Default|GetVehicle)) (* ActionValue (Variables|/Game/Rik/Blueprints/BP_BaseVehicle.BP_BaseVehicle_C|GetMaximumSpeed (Variables|Default|GetVehicle))) (Utilities|Time|GetWorldDeltaSeconds) 4.0))))

(event EventBeginPlay
  (Input|AddMappingContext (PlayerController|LocalPlayerSubsystems|GetEnhancedInputLocalPlayerSubsystem) "/Game/Rik/Input/IMC_Default.IMC_Default" 0 "(bIgnoreAllPressedKeysUntilRelease=True,bForceImmediately=False)")
  (bind _asbp_base_vehicle (Utilities|Casting|CastToBP_BaseVehicle (Pawn|GetControlledPawn)))
  (Variables|Default|SetVehicle _asbp_base_vehicle))

(event EventTick
  (params (DeltaSeconds :type Float%20%28single-precision%29)))

(fn ConstructionScript)