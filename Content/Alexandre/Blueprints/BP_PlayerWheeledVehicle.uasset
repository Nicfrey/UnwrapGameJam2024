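; Player-driven wheeled vehicle that accelerates automatically while the player steers, with health, fuel and wheel health draining over time.
; Each tick applies input, decrements the three clamped attributes, then evaluates their effects.
; Below half health, throttle and engine volume scale down; below half wheel health, a sine wobble of growing amplitude disturbs steering.
; Running out of fuel opens the end screen level.
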(event EventBeginPlay
  (CallFunction|InitAttributes)
  (bind _asplayer_controller (Utilities|Casting|CastToPlayerController (Pawn|GetController)))
  (Utilities|IsValid (PlayerController|LocalPlayerSubsystems|GetEnhancedInputLocalPlayerSubsystem _asplayer_controller)
    (:Is%20Valid
      (Input|AddMappingContext (PlayerController|LocalPlayerSubsystems|GetEnhancedInputLocalPlayerSubsystem _asplayer_controller) "/Game/Alexandre/Blueprints/MC_Movement.MC_Movement" 0 "(bIgnoreAllPressedKeysUntilRelease=True,bForceImmediately=False)"))))

(event Collision|EventActorBeginOverlap
  (params (OtherActor :type Actor%20Object%20Reference)))

(event EventTick
  (params (DeltaSeconds :type Float%20%28single-precision%29))
  (bind _vehiclemovementcomponent (Variables|Default|GetVehicleMovementComponent))
  (Class|ChaosVehicleMovementComponent|SetThrottleInput _vehiclemovementcomponent 1.0)
  (Class|ChaosVehicleMovementComponent|SetSteeringInput _vehiclemovementcomponent (+ (Input|EnhancedActionValues|GetIA_Movement) (Variables|Default|GetRandomAngleVariation)))
  (CallFunction|DecrementAttributes)
  (CallFunction|CheckAttributesValues))

(fn ConstructionScript)

(fn GetHealthPercentage
  (return (/ (Variables|Attributes|GetCurrentVehicleHealth) (Variables|Attributes|GetMaxVehicleHealth))))

(fn GetFuelPercentage
  (return (/ (Variables|Attributes|GetCurrentVehicleFuel) (Variables|Attributes|GetMaxVehicleFuel))))

(fn GetWheelHealthPercentage
  (return (/ (Variables|Attributes|GetCurrentWheelHealth) (Variables|Attributes|GetMaxWheelHealth))))

(fn InitAttributes
  (Variables|Attributes|SetCurrentVehicleHealth (Variables|Attributes|GetMaxVehicleHealth))
  (Variables|Attributes|SetCurrentVehicleFuel (Variables|Attributes|GetMaxVehicleFuel))
  (Variables|Attributes|SetCurrentWheelHealth (Variables|Attributes|GetMaxWheelHealth)))

(fn DecrementAttributes
  (CallFunction|ChangeHealth (* (* (Variables|Attributes|GetHealthLoosingSpeed) (Utilities|Time|GetWorldDeltaSeconds)) -1.0))
  (CallFunction|ChangeFuelValue (* (* (Variables|Attributes|GetFuelLoosingSpeed) (Utilities|Time|GetWorldDeltaSeconds)) -1.0))
  (CallFunction|ChangeWheelHealth (* (* (Variables|Attributes|GetWheelHealthLoosingSpeed) (Utilities|Time|GetWorldDeltaSeconds)) -1.0)))

(fn ChangeHealth
  (params (InitialValue :type Float%20%28double-precision%29))
  (Variables|Attributes|SetCurrentVehicleHealth (+ InitialValue (Variables|Attributes|GetCurrentVehicleHealth)))
  (Utilities|FlowControl|Sequence
    (:then_0
      (if (< (Variables|Attributes|GetCurrentVehicleHealth) 0.0)
        (Variables|Attributes|SetCurrentVehicleHealth 0.0)))
    (:then_1
      (if (> (Variables|Attributes|GetCurrentVehicleHealth) (Variables|Attributes|GetMaxVehicleHealth))
        (Variables|Attributes|SetCurrentVehicleHealth (Variables|Attributes|GetMaxVehicleHealth))))))

(fn ChangeFuelValue
  (params (InitialValue :type Float%20%28double-precision%29))
  (Variables|Attributes|SetCurrentVehicleFuel (+ InitialValue (Variables|Attributes|GetCurrentVehicleFuel)))
  (Utilities|FlowControl|Sequence
    (:then_0
      (if (< (Variables|Attributes|GetCurrentVehicleFuel) 0.0)
        (Variables|Attributes|SetCurrentVehicleFuel 0.0)))
    (:then_1
      (if (> (Variables|Attributes|GetCurrentVehicleFuel) (Variables|Attributes|GetMaxVehicleFuel))
        (Variables|Attributes|SetCurrentVehicleFuel (Variables|Attributes|GetMaxVehicleFuel))))))

(fn ChangeWheelHealth
  (params (InitialValue :type Float%20%28double-precision%29))
  (Variables|Attributes|SetCurrentWheelHealth (+ InitialValue (Variables|Attributes|GetCurrentWheelHealth)))
  (Utilities|FlowControl|Sequence
    (:then_0
      (if (< (Variables|Attributes|GetCurrentWheelHealth) 0.0)
        (Variables|Attributes|SetCurrentWheelHealth 0.0)))
    (:then_1
      (if (> (Variables|Attributes|GetCurrentWheelHealth) (Variables|Attributes|GetMaxWheelHealth))
        (Variables|Attributes|SetCurrentWheelHealth (Variables|Attributes|GetMaxWheelHealth))))))

(fn CheckAttributesValues
  (bind _currentvehiclehealth (Variables|Attributes|GetCurrentVehicleHealth))
  (bind _maxvehiclehealth (Variables|Attributes|GetMaxVehicleHealth))
  (bind _currentvehiclehealth_2 (Variables|Attributes|GetCurrentVehicleHealth))
  (bind _maxvehiclehealth_2 (Variables|Attributes|GetMaxVehicleHealth))
  (bind _returnvalue (/ _maxvehiclehealth 2.0))
  (bind _returnvalue_2 (/ _maxvehiclehealth_2 2.0))
  (bind _returnvalue_3 (> _currentvehiclehealth_2 _returnvalue_2))
  (bind _returnvalue_4 (/ _currentvehiclehealth _returnvalue))
  (bind _returnvalue_5 (Math|Float|SelectFloat 1.0 _returnvalue_4 _returnvalue_3))
  (Utilities|FlowControl|Sequence
    (:then_0
      ;[1 1 1] Out Of Fuel
      (if (<= (Variables|Attributes|GetCurrentVehicleFuel) 0.0)
        (Game|OpenLevel(byName) "ShowEndScreen")))
    (:then_1
      (Class|ChaosVehicleMovementComponent|SetThrottleInput (Variables|Default|GetVehicleMovementComponent) _returnvalue_5)
      (Audio|Components|Audio|SetVolumeMultiplier (Variables|Default|GetEngineSound) _returnvalue_5 :!class /Script/Engine.AudioComponent))
    (:then_2
      ;[1 1 1] Wheel Health
      (Variables|Default|SetRandomAngleVariation (Math|Float|SelectFloat 0.0 (* (Math|Trig|Sin(Radians) (* (Actor|GetGameTimeSinceCreation) 5.0)) (/ 1.0 (/ (Variables|Attributes|GetCurrentWheelHealth) (/ (Variables|Attributes|GetMaxWheelHealth) 2.0)))) (> (Variables|Attributes|GetCurrentWheelHealth) (/ (Variables|Attributes|GetMaxWheelHealth) 2.0)))))))