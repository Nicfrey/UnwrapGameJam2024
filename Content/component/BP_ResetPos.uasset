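; Car component that teleports its owner to a nearby reset point when the car is stuck.
; On BeginPlay it caches every BP_CarResetPoint actor, then enables stuck detection after a short delay.
; ResetPosIfStuck takes a speed from its caller and treats a low but non-zero range as stuck.
; It then searches the cached points by distance and applies the closest one's transform to the owner.
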(event EventBeginPlay
  (bind _outactors (Actor|GetAllActorsOfClass "/Game/component/BP_CarResetPoint.BP_CarResetPoint_C"))
  (Variables|Default|SetresetPoints _outactors)
  (Utilities|FlowControl|Delay 0.5)
  (Variables|Default|SetisStarted true))

(event EventTick
  (params (DeltaSeconds :type Float%20%28single-precision%29)))

(fn ResetPosifStuck
  (params (speed :type Float%20%28double-precision%29))
  (bind _returnvalue (Components|GetOwner))
  (bind _isstuck (CallFunction|IsStuck speed))
  (if _isstuck
    (bind _newparam (CallFunction|GetClosestResetPoint (Transformation|GetActorLocation _returnvalue)))
    (Transformation|SetActorTransform _returnvalue _newparam false true)))

(fn IsStuck
  (params (Speed :type Float%20%28double-precision%29))
  (if (Variables|Default|GetisStarted)
    (return (Math|Float|InRange(Float) Speed 0.5 5.0))))

(fn GetClosestResetPoint
  (params (carLocation :type Vector))
  (for _array_element (Variables|Default|GetresetPoints)
    (if (< (Math|Vector|Distance(Vector) carLocation (Transformation|GetActorLocation _array_element)) (Variables|Default|GetminimumDistance))
      (Variables|Default|SetminimumDistance (Math|Vector|Distance(Vector) carLocation (Transformation|GetActorLocation _array_element)))
      (Variables|Default|SetnewTransform (Transformation|GetActorTransform _array_element))))
  (return (Variables|Default|GetnewTransform)))