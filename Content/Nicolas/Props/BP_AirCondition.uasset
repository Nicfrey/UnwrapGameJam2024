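; BP_AirCondition is an air conditioner prop with a Niagara effect that vehicles can knock loose.
; Construction picks a random mesh and sets prop and effect offsets from a separately evaluated random pick, so offsets can mismatch the mesh.
; A BP_WheeledVehicle overlapping the Box turns on the prop's physics simulation.
; Tick deactivates the Niagara effect once the actor's velocity exceeds a threshold.
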(event OnComponentHit(Prop)
  (params (HitComponent :type Primitive%20Component%20Object%20Reference) (OtherActor :type Actor%20Object%20Reference) (OtherComp :type Primitive%20Component%20Object%20Reference) (NormalImpulse :type Vector :default "0, 0, 0") (Hit :type Hit%20Result%20Structure%20%28by%20ref%29)))

(event OnComponentBeginOverlap(Box)
  (params (OverlappedComponent :type Primitive%20Component%20Object%20Reference) (OtherActor :type Actor%20Object%20Reference) (OtherComp :type Primitive%20Component%20Object%20Reference) (OtherBodyIndex :type Integer) (bFromSweep :type Boolean) (SweepResult :type Hit%20Result%20Structure%20%28by%20ref%29))
  (Utilities|Casting|CastToBP_WheeledVehicle OtherActor)
  (Physics|SetSimulatePhysics (Variables|Default|GetProp) true))

(event EventBeginPlay
  (|CallParentFunction) ; This node is disabled and will not be called.\nDrag off pins to build functionality.
)

(event Collision|EventActorBeginOverlap
  (params (OtherActor :type Actor%20Object%20Reference))
  (|CallParentFunction OtherActor) ; This node is disabled and will not be called.\nDrag off pins to build functionality.
)

(event EventTick
  (params (DeltaSeconds :type Float%20%28single-precision%29))
  (|CallParentFunction DeltaSeconds)
  (if (> (Math|Vector|VectorLength (Transformation|GetVelocity)) 1e+02)
    (Components|Activation|Deactivate (Variables|Default|GetNiagara))))

(fn ConstructionScript
  (bind _meshes (LocalVariables|GetMeshes))
  (bind _niagara (Variables|Default|GetNiagara))
  (bind _returnvalue (Utilities|Array|Length _meshes))
  (bind _returnvalue_2 (- _returnvalue 1))
  (bind _returnvalue_3 (Math|Random|RandomIntegerinRange 0 _returnvalue_2))
  (bind _output (Utilities|Array|Get(acopy) _meshes _returnvalue_3))
  (|CallParentFunction)
  (Components|StaticMesh|SetStaticMesh (Variables|Default|GetProp) _output)
  (if (== _output (Utilities|Array|Get(acopy) (LocalVariables|GetMeshes)))
    (Transformation|SetRelativeLocation _niagara "40.000000,0.000000,0.000000" false false)
    (Transformation|SetRelativeLocation (Variables|Default|GetProp) "0.000000,0.000000,70.000000" false false)
    (else
      (Transformation|SetRelativeLocation _niagara "30.000000,0.000000,0.000000" false false)
      (Transformation|SetRelativeLocation (Variables|Default|GetProp) "0.000000,0.000000,30.000000" false false))))