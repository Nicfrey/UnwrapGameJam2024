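; BP_Bench is a bench prop actor that varies its appearance by picking a random mesh.
; Its construction script sets the Prop static mesh component to a random entry from the NewMesh array.
; The pick is unseeded, so it can change whenever the construction script reruns.
; The event graph holds only disabled default events, so it adds no runtime logic.
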(event EventBeginPlay
  (|CallParentFunction) ; This node is disabled and will not be called.\nDrag off pins to build functionality.
)

(event Collision|EventActorBeginOverlap
  (params (OtherActor :type Actor%20Object%20Reference))
  (|CallParentFunction OtherActor) ; This node is disabled and will not be called.\nDrag off pins to build functionality.
)

(event EventTick
  (params (DeltaSeconds :type Float%20%28single-precision%29))
  (|CallParentFunction DeltaSeconds) ; This node is disabled and will not be called.\nDrag off pins to build functionality.
)

(fn ConstructionScript
  (bind _new_mesh (Variables|Default|GetNew%20Mesh))
  (|CallParentFunction)
  (Components|StaticMesh|SetStaticMesh (Variables|Default|GetProp) (Utilities|Array|Get(acopy) _new_mesh (Math|Random|RandomIntegerinRange 0 (- (Utilities|Array|Length _new_mesh) 1)))))