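; Base Blueprint for props that get knocked flying when a wheeled vehicle hits them.
; When the Prop component is hit by a BP_WheeledVehicle, it receives an impulse along the vehicle's normalized horizontal velocity, plus a random upward kick.
; X and Y strengths are randomized separately, so launch direction scatters slightly.
; The impulse is not a velocity change, so the prop's mass affects the launch.
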(event OnComponentHit(Prop)
  (params (HitComponent :type Primitive%20Component%20Object%20Reference) (OtherActor :type Actor%20Object%20Reference) (OtherComp :type Primitive%20Component%20Object%20Reference) (NormalImpulse :type Vector :default "0, 0, 0") (Hit :type Hit%20Result%20Structure%20%28by%20ref%29))
  (bind _asbp_wheeled_vehicle (Utilities|Casting|CastToBP_WheeledVehicle OtherActor))
  (Physics|AddImpulse (Variables|Default|GetProp) (Math|Vector|MakeVector (* (.x (Math|Vector|Normalize (Transformation|GetVelocity _asbp_wheeled_vehicle))) (Math|Random|RandomFloatinRange 8e+03 1.2e+04)) (* (.y (Math|Vector|Normalize (Transformation|GetVelocity _asbp_wheeled_vehicle))) (Math|Random|RandomFloatinRange 8e+03 1.2e+04)) (Math|Random|RandomFloatinRange 4e+03 8e+03)) "None" false))

(event EventBeginPlay)

(event Collision|EventActorBeginOverlap
  (params (OtherActor :type Actor%20Object%20Reference)))

(event EventTick
  (params (DeltaSeconds :type Float%20%28single-precision%29)))

(fn ConstructionScript)