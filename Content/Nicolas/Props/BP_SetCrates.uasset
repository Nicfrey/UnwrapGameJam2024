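; BP_SetCrates is a breakable crate-stack prop that bursts into small crates when a wheeled vehicle overlaps its box.
; The construction script randomizes the stack mesh and small-crate type, tinting one variant, though separate random rolls can mismatch them.
; On overlap it spawns a random number of BP_Crates, pushes them along the car's velocity and hides its mesh.
; After a delay, it destroys the spawned crates and itself.
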(event OnComponentBeginOverlap(Box)
  (params (OverlappedComponent :type Primitive%20Component%20Object%20Reference) (OtherActor :type Actor%20Object%20Reference) (OtherComp :type Primitive%20Component%20Object%20Reference) (OtherBodyIndex :type Integer) (bFromSweep :type Boolean) (SweepResult :type Hit%20Result%20Structure%20%28by%20ref%29))
  (bind _returnvalue (Transformation|GetActorTransform))
  (bind _asbp_wheeled_vehicle (Utilities|Casting|CastToBP_WheeledVehicle OtherActor))
  (Variables|Default|SetDirectionCar (Math|Vector|Normalize (Transformation|GetVelocity _asbp_wheeled_vehicle)))
  (bind _output_get (Variables|Default|SetNbSpawnCrate (Math|Random|RandomIntegerinRange (Variables|Default|GetMinSpawnCrate) (Variables|Default|GetMaxSpawnCrate))))
  (for _index (range 0 _output_get)
    (bind _returnvalue_2 (Game|SpawnActorfromClass "/Game/Nicolas/Props/BP_Crates.BP_Crates_C" (Math|Transform|MakeTransform (Math|Vector|MakeVector (.x (.location _returnvalue)) (.y (.location _returnvalue)) (Math|Random|RandomFloatinRange 0.0 5e+01)) (.rotation _returnvalue) "1.000000,1.000000,1.000000") "Undefined" "MultiplyWithRoot" 0 0))
    (Components|StaticMesh|SetStaticMesh (Variables|/Game/Nicolas/Props/BP_PropsBase.BP_PropsBase_C|GetProp _returnvalue_2) (Variables|Default|GetSmallCrate))
    (Physics|AddImpulse (Variables|/Game/Nicolas/Props/BP_PropsBase.BP_PropsBase_C|GetProp _returnvalue_2) (* (Variables|Default|GetDirectionCar) 5e+02) "None" false)
    (Utilities|Array|Add (Variables|Default|GetCrates) _returnvalue_2))
  (Development|SetHiddeninGame (Variables|Default|GetProp) true false)
  (Utilities|FlowControl|Delay 1e+01)
  (for _array_element (Variables|Default|GetCrates)
    (Actor|DestroyActor _array_element))
  (Actor|DestroyActor))

(event EventBeginPlay
  (|CallParentFunction) ; This node is disabled and will not be called.\nDrag off pins to build functionality.
)

(event Collision|EventActorBeginOverlap
  (params (OtherActor :type Actor%20Object%20Reference))
  (|CallParentFunction OtherActor) ; This node is disabled and will not be called.\nDrag off pins to build functionality.
)

(event EventTick
  (params (DeltaSeconds :type Float%20%28single-precision%29))
  (|CallParentFunction DeltaSeconds) ; This node is disabled and will not be called.\nDrag off pins to build functionality.
)

(fn ConstructionScript
  (bind _meshes (LocalVariables|GetMeshes))
  (bind _prop (Variables|Default|GetProp))
  (bind _returnvalue (Utilities|Array|Length _meshes))
  (bind _returnvalue_2 (- _returnvalue 1))
  (bind _returnvalue_3 (Math|Random|RandomIntegerinRange 0 _returnvalue_2))
  (|CallParentFunction)
  (LocalVariables|Setindex _returnvalue_3)
  (Components|StaticMesh|SetStaticMesh (Variables|Default|GetProp) (Utilities|Array|Get(acopy) _meshes _returnvalue_3))
  (Development|PrintString "Hello")
  (switch int (LocalVariables|Getindex)
    (:0
      (Variables|Default|SetSmallCrate "/Game/AssetsvilleTown/Meshes/StreetProps/SM_crate_1.SM_crate_1"))
    (:1
      (Variables|Default|SetSmallCrate "/Game/AssetsvilleTown/Meshes/StreetProps/SM_crate_1.SM_crate_1")
      (bind _returnvalue_4 (Rendering|Material|CreateDynamicMaterialInstance _prop 0 "/Game/Materials/M_BaseMaterial.M_BaseMaterial" "None" :!class /Script/Engine.PrimitiveComponent))
      (Rendering|Material|SetVectorParameterValue _returnvalue_4 "Color" "(R=0.215861,G=0.031896,B=0.024158,A=1.000000)" :!class /Script/Engine.MaterialInstanceDynamic)
      (Rendering|Material|SetMaterial _prop 0 _returnvalue_4))
    (:2
      (Variables|Default|SetSmallCrate "/Game/AssetsvilleTown/Meshes/StreetProps/SM_crate_3.SM_crate_3"))
    (:3
      (Variables|Default|SetSmallCrate "/Game/AssetsvilleTown/Meshes/StreetProps/SM_crate_4.SM_crate_4"))))