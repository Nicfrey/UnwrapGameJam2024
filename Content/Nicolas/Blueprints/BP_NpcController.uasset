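; AI controller for an NPC that flags it to flee when it perceives the player.
; On BeginPlay it sets up the BB_Npc blackboard and runs the BT_Npc behavior tree.
; Sensing the player pawn sets PlayerSeen and Fleeing and stores the pawn as Car.
; Any other perception update, including a lost stimulus, clears only PlayerSeen, leaving Fleeing set.
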(event OnTargetPerceptionUpdated(AIPerception)
  (params (Actor :type Actor%20Object%20Reference) (Stimulus :type AI%20Stimulus%20Structure))
  (bind _returnvalue (AI|GetBlackboard 0))
  (bind _returnvalue_2 (Game|Player|GetPlayerPawn 0))
  (if (.bsuccessfullysensed Stimulus)
    (if (== Actor _returnvalue_2)
      (AI|Components|Blackboard|SetValueasBool (AI|GetBlackboard 0) (Utilities|Name|MakeLiteralName "PlayerSeen") true)
      (AI|Components|Blackboard|SetValueasBool _returnvalue (Utilities|Name|MakeLiteralName "Fleeing") true)
      (AI|Components|Blackboard|SetValueasObject _returnvalue (Utilities|Name|MakeLiteralName "Car") _returnvalue_2)
      (else
        (AI|Components|Blackboard|SetValueasBool (AI|GetBlackboard 0) (Utilities|Name|MakeLiteralName "PlayerSeen") false :!label _label)))
    (else
      (goto _label))))

(event EventBeginPlay
  (Class|AIController|UseBlackboard "/Game/Nicolas/Blueprints/BB_Npc.BB_Npc")
  (AI|RunBehaviorTree "/Game/Nicolas/Blueprints/BT_Npc.BT_Npc"))

(event EventTick
  (params (DeltaSeconds :type Float%20%28single-precision%29)))

(fn ConstructionScript)