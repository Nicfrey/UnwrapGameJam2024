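; Behavior tree task that makes an NPC flee from the actor stored in the "Car" blackboard key.
; It asks the NPC character for a fleeing location relative to that actor and moves there with AI MoveTo.
; On arrival it clears the "Fleeing" blackboard flag and finishes successfully; failed moves or casts never call FinishExecute.
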(event EventReceiveExecuteAI
  (params (OwnerController :type AI%20Controller%20Object%20Reference) (ControlledPawn :type Pawn%20Object%20Reference))
  (bind _asbp_npc_character (Utilities|Casting|CastToBP_NpcCharacter ControlledPawn))
  (bind _asbp_npc_controller (Utilities|Casting|CastToBP_NpcController OwnerController))
  (bind _asactor (Utilities|Casting|CastToActor (AI|Components|Blackboard|GetValueasObject (AI|GetBlackboard _asbp_npc_controller) (Utilities|Name|MakeLiteralName "Car"))))
  (AI|AIMoveTo _asbp_npc_character (Default|GetFleeingLocation _asbp_npc_character _asactor) 0 5.0 false
    (:OnSuccess
      (AI|Components|Blackboard|SetValueasBool (AI|GetBlackboard _asbp_npc_controller) (Utilities|Name|MakeLiteralName "Fleeing") false)
      (AI|BehaviorTree|FinishExecute true))))