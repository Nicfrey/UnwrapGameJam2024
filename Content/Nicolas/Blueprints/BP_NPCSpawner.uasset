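; Spawner actor that populates an area with AI-controlled BP_NpcCharacter pawns running the BT_Npc behavior tree.
; The Construction Script sizes and offsets the box from BoxExtent, then appends random points until SpawnPoints matches a non-zero NbsNPCs, without clearing existing ones.
; Points span one BoxExtent from the actor in X and Y at a fixed world Z, covering only part of the box.
; BeginPlay spawns one NPC at each point.
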(event EventBeginPlay
  (for _array_element (Variables|Default|GetSpawnPoints)
    (AI|SpawnAIFromClass "/Game/Nicolas/Blueprints/BP_NpcCharacter.BP_NpcCharacter_C" "/Game/Nicolas/Blueprints/BT_Npc.BT_Npc" _array_element "0, 0, 0" false 0)))

(event Collision|EventActorBeginOverlap
  (params (OtherActor :type Actor%20Object%20Reference)))

(event EventTick
  (params (DeltaSeconds :type Float%20%28single-precision%29)))

(fn ConstructionScript
  (bind _returnvalue (Transformation|GetActorLocation))
  (bind _nbsnpcs (Variables|Default|GetNbsNPCs))
  (bind _boxextent (Variables|Default|GetBoxExtent))
  (bind _boxextent_2 (Variables|Default|GetBoxExtent))
  (bind _box (Variables|Default|GetBox))
  (Components|Box|SetBoxExtent _box (Variables|Default|GetBoxExtent) true)
  (Transformation|SetRelativeLocation _box (Math|Vector|MakeVector (.x _boxextent) (.y _boxextent) 0.0) false false)
  (if (!= _nbsnpcs 0)
    (while (!= _nbsnpcs (Utilities|Array|Length (Variables|Default|GetSpawnPoints)))
      (Utilities|Array|Add (Variables|Default|GetSpawnPoints) (Math|Vector|MakeVector (Math|Random|RandomFloatinRange (.x _returnvalue) (+ (.x _returnvalue) (.x _boxextent_2))) (Math|Random|RandomFloatinRange (.y _returnvalue) (+ (.y _returnvalue) (.y _boxextent_2))) 1e+01)))))