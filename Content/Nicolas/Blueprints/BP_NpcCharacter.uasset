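; BP_NpcCharacter is an NPC character that walks, flees from cars and ragdolls when run over.
; Construction picks a random skeletal mesh, and a looping timer switches walk or run speed from the Blackboard "Fleeing" key.
; Overlap with a BP_WheeledVehicle marks it dead, launches the ragdoll along the car's forward vector, then destroys it after a delay.
; Helper functions supply random and away-from-car destinations and the death state.
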(event OnComponentBeginOverlap(DetectCar)
  (params (OverlappedComponent :type Primitive%20Component%20Object%20Reference) (OtherActor :type Actor%20Object%20Reference) (OtherComp :type Primitive%20Component%20Object%20Reference) (OtherBodyIndex :type Integer) (bFromSweep :type Boolean) (SweepResult :type Hit%20Result%20Structure%20%28by%20ref%29))
  (bind _mesh (Variables|Character|GetMesh))
  (bind _asbp_wheeled_vehicle (Utilities|Casting|CastToBP_WheeledVehicle OtherActor))
  (Variables|Default|SetDead? true)
  (Collision|SetCollisionResponsetoAllChannels (Variables|Collision|GetCapsuleComponent) "ECR_Ignore")
  (Class|SkeletalMeshComponent|SetAllBodiesBelowSimulatePhysics _mesh (Class|SkinnedMeshComponent|GetBoneName (Variables|Character|GetMesh)) true true)
  (Class|SkeletalMeshComponent|AddImpulsetoAllBodiesBelow _mesh (Math|Vector|MakeVector (* (.x (Transformation|GetActorForwardVector _asbp_wheeled_vehicle)) (Math|Random|RandomFloatinRange 1e+04 2e+04)) (* (.y (Transformation|GetActorForwardVector _asbp_wheeled_vehicle)) (Math|Random|RandomFloatinRange 1e+04 2e+04)) (Math|Random|RandomFloatinRange 6e+03 1e+04)) "None" false true)
  (Utilities|FlowControl|Delay 1e+01)
  (Actor|DestroyActor))

(event Custom|ChangeSpeed
  (bind _charactermovement (Variables|Character|GetCharacterMovement))
  (if (ScalableFloat|GetValueasBool (AI|GetBlackboard 0) (Utilities|Name|MakeLiteralName "Fleeing"))
    (Variables|/Script/Engine.CharacterMovementComponent|SetMaxWalkSpeed _charactermovement (Variables|Default|GetMaxSpeedRunning))
    (else
      (Variables|/Script/Engine.CharacterMovementComponent|SetMaxWalkSpeed _charactermovement (Variables|Default|GetMaxSpeedWalking)))))

(event EventBeginPlay
  (Variables|/Script/Engine.CharacterMovementComponent|SetMaxWalkSpeed (Variables|Character|GetCharacterMovement) (Variables|Default|GetMaxSpeedWalking))
  (Utilities|Time|SetTimerbyEvent (delegate Custom|ChangeSpeed) 0.5 true)
  (Utilities|Time|SetTimerbyEvent 0 0.5 true))

(event Collision|EventActorBeginOverlap
  (params (OtherActor :type Actor%20Object%20Reference)))

(event EventTick
  (params (DeltaSeconds :type Float%20%28single-precision%29)))

(fn ConstructionScript
  (bind _new_mesh (Variables|Default|GetNew%20Mesh))
  (Components|SkeletalMesh|SetSkeletalMeshAsset (Variables|Character|GetMesh) (Utilities|Array|Get(acopy) _new_mesh (Math|Random|RandomIntegerinRange 0 (- (Utilities|Array|Length _new_mesh) 1)))))

(fn GetRandomLocation
  (bind _returnvalue (Math|Random|RandomFloatinRange 0.0 3.6e+02))
  (return (+ (Math|Vector|MakeVector (* (Math|Trig|Cos(Degrees) _returnvalue) (Variables|Default|GetRadiusLocation)) (* (Math|Trig|Sin(Degrees) _returnvalue) (Variables|Default|GetRadiusLocation)) 0.0) (Transformation|GetActorLocation))))

(fn GetFleeingLocation
  (params (Car :type Actor%20Object%20Reference))
  (bind _returnvalue (Transformation|GetActorLocation))
  (bind _returnvalue_2 (Transformation|GetActorLocation Car))
  (bind _returnvalue_3 (- _returnvalue _returnvalue_2))
  (bind _returnvalue_4 (Math|Vector|Normalize _returnvalue_3))
  (return (+ (Transformation|GetActorLocation) (Math|Vector|MakeVector (* (.x _returnvalue_4) 5e+02) (* (.y _returnvalue_4) 5e+02) 0.0))))

(fn IsDead
  (return (Variables|Default|GetDead?)))