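; BP_SpawnPickupComponent is a component that fills the level's pickup points with random pickups and respawns them on request.
; On BeginPlay it gathers every BP_SpawnPickUpPoint and spawns a class picked at random from SpawnObjects at each one.
; Its StartPickup event takes a location, waits TimeToSpawn, then spawns a new random pickup there.
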(event EventBeginPlay
  (Development|PrintString "component says hello")
  (bind _outactors (Actor|GetAllActorsOfClass "/Game/PickUps/BP_SpawnPickUpPoint.BP_SpawnPickUpPoint_C"))
  (Variables|Default|SetspawnPoints _outactors)
  ;[1 1 1] Spawn a random item on all pickup points
  (CallFunction|SpawnonAllPoints))

(event EventTick
  (params (DeltaSeconds :type Float%20%28single-precision%29)))

(event EventStartPickup
  (params (location :type Vector :default "0, 0, 0"))
  (Utilities|FlowControl|Delay (Variables|Default|GettimeToSpawn))
  (CallFunction|Spawn location))

(fn Spawn
  (params (spawnLocation :type Vector))
  (CallFunction|GetRandomObject)
  (Game|SpawnActorfromClass (Variables|Default|GetrandomPickup) (Math|Transform|MakeTransform spawnLocation "0, 0, 0" "1.000000,1.000000,1.000000") "Undefined" "MultiplyWithRoot" 0 0))

(fn SpawnonAllPoints
  (for _array_element (Variables|Default|GetspawnPoints)
    (CallFunction|GetRandomObject)
    (Game|SpawnActorfromClass (Variables|Default|GetrandomPickup) (Math|Transform|MakeTransform (Transformation|GetActorLocation _array_element) "0, 0, 0" "1.000000,1.000000,1.000000") "AlwaysSpawn" "MultiplyWithRoot" 0 0)))

(fn GetRandomObject
  (Variables|Default|SetrandomPickup (.OutItem (Utilities|Array|Random (Variables|Default|GetspawnObjects)))))